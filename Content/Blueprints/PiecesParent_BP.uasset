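; Base chess piece actor, configured by PieceID as king, queen, bishop, horse, rook or pawn, and by Side as black or white.
; The construction script sets mesh, capsule size, component offsets, team material and some wave effects.
; A dynamic material drives the outline color, with Tick polling flags to refresh it or spawn teleport sparks.
; Destruction spawns a particle burst, and a destroyed king shows the EndGame widget naming the opposing team as winner.
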(event EventTick
  (params (DeltaSeconds :type Float%20%28single-precision%29))
  (Utilities|FlowControl|Sequence
    (:then_0
      (if (Variables|Default|GetRefreshOutline)
        (Utilities|FlowControl|DoOnce false :!label _label
          (:Completed
            (Rendering|Material|SetVectorParameterValue (Variables|Default|GetOutline) "OutlineColor" (Variables|Default|GetOutlineColor) :!class /Script/Engine.MaterialInstanceDynamic)
            (Variables|Default|SetRefreshOutline false)
            (goto _label Reset)))))
    (:then_1
      (if (Variables|Default|GetTeleportParticle)
        (Utilities|FlowControl|DoOnce false :!label _label_2
          (:Completed
            (Effects|SpawnEmitteratLocation "/Game/Assets/Explosions/Particles/P_SparksFlair.P_SparksFlair" (Transformation|GetActorLocation) "90.000000, 0, 0")
            (Variables|Default|SetTeleportParticle false)
            (goto _label_2 Reset)))))))

(event EventBeginPlay
  (bind _destructible (Variables|Default|GetDestructible))
  (bind _returnvalue (Rendering|Material|CreateDynamicMaterialInstance (Rendering|Material|GetMaterial _destructible 0) :!class /Script/Engine.KismetMaterialLibrary))
  (Rendering|Material|SetMaterial _destructible 0 _returnvalue)
  (Variables|Default|SetOutline _returnvalue))

(event EventDestroyed
  (Effects|SpawnEmitteratLocation "/Game/Assets/InfinityBladeEffects/Effects/FX_Combat_Base/WeaponCombo/P_Cube_Mesh_Test.P_Cube_Mesh_Test" (Transformation|GetActorLocation) (Transformation|GetActorRotation))
  (if (== 0 (Variables|Default|GetPieceID))
    (bind _returnvalue (UserInterface|CreateWidget "/Game/Widgets/EndGame.EndGame_C" (Game|GetPlayerController 0)))
    (Utilities|IsValid _returnvalue
      (:Is%20Valid
        (UserInterface|Viewport|AddtoViewport _returnvalue 0)
        (if (Variables|Default|GetSide)
          (Rendering|Components|TextRender|SetText (Variables|/Game/Widgets/EndGame.EndGame_C|GetWinnerTeam _returnvalue) "White")
          (else
            (Rendering|Components|TextRender|SetText (Variables|/Game/Widgets/EndGame.EndGame_C|GetWinnerTeam _returnvalue) "Black")))))))

(fn ConstructionScript
  (Utilities|FlowControl|Sequence
    (:then_0
      (switch int (Variables|Default|GetPieceID)
        (:0
          (Components|StaticMesh|SetStaticMesh (Variables|Default|GetDestructible) "/Game/Assets/ChessPieces/LowPolySet/King.King")
          (Utilities|SetCapsule 25.0 75.0 "0.000000,0,-70.000000")
          (Transformation|SetRelativeRotation (Variables|Default|GetDestructible) "0,90.000000, 0" false false))
        (:1
          (Components|StaticMesh|SetStaticMesh (Variables|Default|GetDestructible) "/Game/Assets/ChessPieces/LowPolySet/Queen.Queen")
          (Utilities|SetCapsule 2e+01 6e+01 "0.000000,0,-60.000000"))
        (:2
          (Components|StaticMesh|SetStaticMesh (Variables|Default|GetDestructible) "/Game/Assets/ChessPieces/LowPolySet/Bishop.Bishop")
          (Utilities|SetCapsule 15.0 5e+01 "0.000000,0,-50.000000")
          (Effects|Components|ParticleSystem|SetTemplate (Variables|Default|GetWave) "/Game/Assets/Explosions/Particles/P_shockwave.P_shockwave")
          (Transformation|SetRelativeRotation (Variables|Default|GetDestructible) "0,180.000000, 0" false false :!label _label)
          (Transformation|SetRelativeRotation (Variables|Default|GetWave) "90.000000, 0, 0" false false :!label _label_2))
        (:3
          (Components|StaticMesh|SetStaticMesh (Variables|Default|GetDestructible) "/Game/Assets/ChessPieces/LowPolySet/Horse.Horse")
          (Utilities|SetCapsule 2e+01 45.0 "0.000000,0,-40.000000")
          (goto _label))
        (:4
          (Components|StaticMesh|SetStaticMesh (Variables|Default|GetDestructible) "/Game/Assets/ChessPieces/LowPolySet/Rook.Rook")
          (Utilities|SetCapsule 2e+01 4e+01 "0.000000,0,-40.000000")
          (Effects|Components|ParticleSystem|SetTemplate (Variables|Default|GetWave) "/Game/Assets/Explosions/Particles/P_shieldwave.P_shieldwave")
          (goto _label_2))
        (:5
          (Components|StaticMesh|SetStaticMesh (Variables|Default|GetDestructible) "/Game/Assets/ChessPieces/LowPolySet/Pawn.Pawn")
          (Utilities|SetCapsule 1e+01 3e+01 "0.000000,0,-30.000000"))))
    (:then_1
      (if (Variables|Default|Getside)
        (Rendering|Material|SetMaterial (Variables|Default|GetDestructible) 0 "/Game/Assets/ChessPieces/GTFreeMaterials/Materials/Black_Mat.Black_Mat")
        (else
          (Rendering|Material|SetMaterial (Variables|Default|GetDestructible) 0 "/Game/Assets/ChessPieces/GTFreeMaterials/Materials/White_Mat.White_Mat"))))))