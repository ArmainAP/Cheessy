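; Base Blueprint for a chess piece, with a destructible mesh and one-shot distortion and teleport effects.
; The construction script uses PieceID to pick the mesh and size the capsule via SetCapsule, which also offsets attached components, then colors it black or white by Side.
; Bishop and rook also get shockwave and shieldwave particle templates respectively.
; Tick polls two boolean flags, spawning the matching emitter and clearing the flag.
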(event EventTick
  (params (DeltaSeconds :type Float%20%28single-precision%29))
  (Utilities|FlowControl|Sequence
    (:then_0
      (if (Variables|Default|GetDistortionParticle)
        (Utilities|FlowControl|DoOnce false :!label _label
          (:Completed
            (bind _returnvalue (Effects|SpawnEmitteratLocation "/Game/Explosions/Particles/P_Distortion3D.P_Distortion3D" (Transformation|GetActorLocation) "90.000000, 0,0.000000"))
            (Transformation|SetWorldScale3D _returnvalue "0.500000,0.150000,0.150000")
            (Variables|Default|SetDistortionParticle false)
            (goto _label Reset)))))
    (:then_1
      (if (Variables|Default|GetTeleportParticle)
        (Utilities|FlowControl|DoOnce false :!label _label_2
          (:Completed
            (Effects|SpawnEmitteratLocation "/Game/Explosions/Particles/P_SparksFlair.P_SparksFlair" (Transformation|GetActorLocation) "90.000000, 0, 0")
            (Variables|Default|SetTeleportParticle false)
            (goto _label_2 Reset)))))))

(fn ConstructionScript
  (Utilities|FlowControl|Sequence
    (:then_0
      (switch int (Variables|Default|GetPieceID)
        (:0
          (Class|DestructibleComponent|SetDestructibleMesh (Variables|Default|GetDestructible) "/Game/ChessPieces/LowPolySet/King_DM.King_DM")
          (Utilities|SetCapsule 25.0 75.0 "0.000000,0,-70.000000"))
        (:1
          (Class|DestructibleComponent|SetDestructibleMesh (Variables|Default|GetDestructible) "/Game/ChessPieces/LowPolySet/Queen_DM.Queen_DM")
          (Utilities|SetCapsule 2e+01 6e+01 "0.000000,0,-60.000000"))
        (:2
          (Class|DestructibleComponent|SetDestructibleMesh (Variables|Default|GetDestructible) "/Game/ChessPieces/LowPolySet/Bishop_DM.Bishop_DM")
          (Utilities|SetCapsule 15.0 5e+01 "0.000000,0,-50.000000")
          (Effects|Components|ParticleSystem|SetTemplate (Variables|Default|GetWave) "/Game/Explosions/Particles/P_shockwave.P_shockwave")
          (Transformation|SetRelativeRotation (Variables|Default|GetDestructible) "0,180.000000, 0" false false :!label _label)
          (Transformation|SetRelativeRotation (Variables|Default|GetWave) "90.000000, 0, 0" false false :!label _label_2))
        (:3
          (Class|DestructibleComponent|SetDestructibleMesh (Variables|Default|GetDestructible) "/Game/ChessPieces/LowPolySet/Horse_DM.Horse_DM")
          (Utilities|SetCapsule 2e+01 45.0 "0.000000,0,-40.000000")
          (goto _label))
        (:4
          (Class|DestructibleComponent|SetDestructibleMesh (Variables|Default|GetDestructible) "/Game/ChessPieces/LowPolySet/Rook_DM.Rook_DM")
          (Utilities|SetCapsule 2e+01 4e+01 "0.000000,0,-40.000000")
          (Effects|Components|ParticleSystem|SetTemplate (Variables|Default|GetWave) "/Game/Explosions/Particles/P_shieldwave.P_shieldwave")
          (goto _label_2))
        (:5
          (Class|DestructibleComponent|SetDestructibleMesh (Variables|Default|GetDestructible) "/Game/ChessPieces/LowPolySet/Pawn_DM.Pawn_DM")
          (Utilities|SetCapsule 1e+01 3e+01 "0.000000,0,-30.000000"))))
    (:then_1
      (if (Variables|Default|Getside)
        (Rendering|Material|SetMaterial (Variables|Default|GetDestructible) 0 "/Game/ChessPieces/GTFreeMaterials/Materials/Black_Mat.Black_Mat")
        (else
          (Rendering|Material|SetMaterial (Variables|Default|GetDestructible) 0 "/Game/ChessPieces/GTFreeMaterials/Materials/White_Mat.White_Mat"))))))