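; MyOnlineGameMode is a game mode that overrides player start selection, apparently for two players in an online match.
; ChoosePlayerStart gathers all PlayerStart actors and returns the first if its tag is "0", retagging it "Taken".
; Otherwise it tags and returns the second without checking its tag, so selection depends on actor array order and every later player gets that start.
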(fn ConstructionScript)

(fn ChoosePlayerStart
  (params (Player :type Controller%20Object%20Reference))
  (bind _outactors (Actor|GetAllActorsOfClass "/Script/Engine.PlayerStart"))
  (if (Utilities|Name|Equal(Name) (Variables|/Script/Engine.PlayerStart|GetPlayerStartTag (Utilities|Array|Get(acopy) _outactors)) "0")
    (Variables|/Script/Engine.PlayerStart|SetPlayerStartTag (Utilities|Array|Get(acopy) _outactors) "Taken")
    (LocalVariables|SetPlayerStart (Utilities|Array|Get(acopy) _outactors))
    (else
      (Variables|/Script/Engine.PlayerStart|SetPlayerStartTag (Utilities|Array|Get(acopy) _outactors 1) "Taken")
      (LocalVariables|SetPlayerStart (Utilities|Array|Get(acopy) _outactors 1))))
  (return (LocalVariables|GetPlayerStart)))