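; Player controller that spawns the player's character, manages the in-game menu and shows the end-of-game screen.
; BeginPlay creates a collapsed menu for the local player, revealed by the Back input, then spawns MyCharacter_BP at a fixed location and possesses it.
; Tick polls ForceWin and, while true, creates a new EndGame widget every frame, naming White or Black as winner from PlayerID.
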(event Custom|Possession
  (bind _returnvalue (Game|SpawnActorfromClass "/Game/Blueprints/MyCharacter_BP.MyCharacter_BP_C" (Math|Transform|MakeTransform "-777.000000, 0,222.000000") "AlwaysSpawn" 0 0))
  (Pawn|Possess _returnvalue))

(event EventBeginPlay
  (bind _self self)
  (Utilities|FlowControl|Sequence
    (:then_0
      (if (Pawn|IsLocalPlayerController _self)
        (bind _returnvalue (UserInterface|CreateWidget "/Game/Widgets/InGameMenu.InGameMenu_C" _self))
        (Utilities|IsValid _returnvalue
          (:Is%20Valid
            (UserInterface|Viewport|AddtoViewport _returnvalue 0)
            (Widget|SetVisibility _returnvalue "Collapsed")))))
    (:then_1
      (CallFunction|Possession))))

(event EventTick
  (params (DeltaSeconds :type Float%20%28single-precision%29))
  (if (Variables|Default|GetForceWin)
    (bind _returnvalue (UserInterface|CreateWidget "/Game/Widgets/EndGame.EndGame_C" (Game|GetPlayerController 0)))
    (Utilities|IsValid _returnvalue
      (:Is%20Valid
        (UserInterface|Viewport|AddtoViewport _returnvalue 0)
        (if (== (Variables|Default|GetPlayerID) 0)
          (Rendering|Components|TextRender|SetText (Variables|/Game/Widgets/EndGame.EndGame_C|GetWinnerTeam _returnvalue) "White")
          (else
            (Rendering|Components|TextRender|SetText (Variables|/Game/Widgets/EndGame.EndGame_C|GetWinnerTeam _returnvalue) "Black")))))))

(event Input|ActionEvents|InputActionBack
  (params (Key :type Key%20Structure :default "AnyKey"))
  (:Pressed
    (Widget|SetVisibility (stale EventBeginPlay _returnvalue) "Visible")))

(fn ConstructionScript)